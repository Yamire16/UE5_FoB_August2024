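; GameStateFOB is a game state that keeps players spawned and tracks the alive count and a zone countdown.
; A looping one-second timer scans PlayerArray for invalid pawns and adjusts PlayersAlive around each respawn.
; Respawning creates a third-person character at a random PlayerStart, possesses it and restores game input and walking.
; A separate Update event, not called in this graph, decrements ZoneTimer after a delay and resets it on expiry.
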(event Custom|CheckPlayerStatus
  (for _array_element (Variables|Default|GetPlayerArray)
    (Utilities|IsValid (PlayerState|GetPawn _array_element)
      (:Is%20Not%20Valid
        (Actor|DestroyActor (PlayerState|GetPawn _array_element))
        (bind _result (Math|Integer|DecrementInt (Variables|Default|GetPlayersAlive))
          (:%20%20
            (Variables|Default|SetPlayersAlive _result)
            (CallFunction|SpawnServerPlayer)))))))

(event Custom|Update
  (Utilities|FlowControl|Delay 1.0)
  (CallFunction|UpdateZoneTimer))

(event Custom|SpawnServerPlayer
  (bind _outactors (Actor|GetAllActorsOfClass "/Script/Engine.PlayerStart"))
  (bind _asbp_fo_b_player_controller (Utilities|Casting|CastToBP_FoB_PlayerController (Game|GetPlayerController (stale Custom|CheckPlayerStatus _array_element))))
  (bind _returnvalue (Game|SpawnActorfromClass "/Game/ThirdPerson/Blueprints/BP_ThirdPersonCharacter.BP_ThirdPersonCharacter_C" (Transformation|GetActorTransform (.OutItem (Utilities|Array|Random _outactors))) "AdjustIfPossibleButAlwaysSpawn" "MultiplyWithRoot" 0 _asbp_fo_b_player_controller 0))
  (bind _result (Math|Integer|IncrementInt (Variables|Default|GetPlayersAlive))
    (:%20%20
      (Variables|Default|SetPlayersAlive _result)
      (Pawn|Possess (Game|GetPlayerController (stale Custom|CheckPlayerStatus _array_element)) _returnvalue)
      (Input|SetInputModeGameOnly (Game|GetPlayerController (stale Custom|CheckPlayerStatus _array_element)) true)
      (Variables|/Script/Engine.PlayerController|SetbShowMouseCursor (Game|GetPlayerController (stale Custom|CheckPlayerStatus _array_element)) false)
      (Variables|/Game/ThirdPerson/Blueprints/BP_ThirdPersonCharacter.BP_ThirdPersonCharacter_C|SetIsDead _returnvalue false)
      (Pawn|Components|CharacterMovement|SetMovementMode (Variables|/Script/Engine.Character|GetCharacterMovement _returnvalue) "MOVE_Walking" 0))))

(event EventBeginPlay
  (bind _returnvalue (Utilities|Time|SetTimerbyEvent (delegate Custom|CheckPlayerStatus) 1.0 true))
  (Variables|Default|SetCheckPlayerH _returnvalue))

(event EventTick
  (params (DeltaSeconds :type Float%20%28single-precision%29)))

(fn ConstructionScript)

(fn UpdateZoneTimer
  (bind _result (Math|Integer|DecrementInt (Variables|Default|GetZone%20Timer))
    (:%20%20
      (if (not (> _result 0))
        (Variables|Default|SetZone%20Timer 10)))))